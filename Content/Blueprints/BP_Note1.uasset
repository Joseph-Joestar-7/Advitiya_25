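; BP_Note1 is an interactable note that shows and hides a full note widget on screen.
; Interact runs a FlipFlop: the first use creates WB_Note2, adds it to the viewport and ignores player look and move input.
; The next use removes the widget and restores that input.
; CanInteract always returns true, so the note is always available.
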(event EventBeginPlay)

(event Collision|EventActorBeginOverlap
  (params (OtherActor :type Actor%20Object%20Reference)))

(event EventTick
  (params (DeltaSeconds :type Float%20%28single-precision%29)))

(event EventInteract
  (params (Interactor :type Actor%20Object%20Reference))
  (bind _returnvalue (Game|GetPlayerController 0))
  (Utilities|FlowControl|FlipFlop
    (:A
      (bind _returnvalue_2 (UserInterface|CreateWidget "/Game/UI/WB_Note2.WB_Note2_C"))
      (UserInterface|Viewport|AddtoViewport _returnvalue_2 0)
      (Input|SetIgnoreLookInput _returnvalue true)
      (Input|SetIgnoreMoveInput _returnvalue true))
    (:B
      (Widget|RemovefromParent _returnvalue_2)
      (Input|SetIgnoreLookInput _returnvalue false)
      (Input|SetIgnoreMoveInput _returnvalue false))))

(fn ConstructionScript)

(fn CanInteract?
  (return true))