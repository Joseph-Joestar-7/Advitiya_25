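; BP_Headphone is an interactable headphone prop that can be repaired through a BPC_Fix component.
; Interact calls the component's Repair, and CanInteract allows interaction only while the component is not yet fixed.
; When HasBeenFixed fires, it calls DoneMessage on the player character, plays a switch sound at its location and clears the overlay material on three circle meshes.
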(event HasBeenFixed(BPC_Fix)
  (Class|BPIPlayer|Done(Message) (Game|GetPlayerCharacter 0))
  (Audio|PlaySoundatLocation "/Engine/VREditor/Sounds/UI/Flashlight_Switch.Flashlight_Switch" (Transformation|GetActorLocation) "0, 0, 0" 1.0 1.0 0.0 0 0 0 0)
  (Rendering|Material|SetOverlayMaterial (Variables|Default|GetCircle_002__0) 0 :!class /Script/Engine.MeshComponent))

(event EventBeginPlay)

(event Collision|EventActorBeginOverlap
  (params (OtherActor :type Actor%20Object%20Reference)))

(event EventTick
  (params (DeltaSeconds :type Float%20%28single-precision%29)))

(event EventInteract
  (params (Interactor :type Actor%20Object%20Reference))
  (Default|Repair (Variables|Default|GetBPC_Fix)))

(fn ConstructionScript)

(fn CanInteract?
  (return (not (Variables|/Game/Blueprints/BPC_Fix.BPC_Fix_C|GetisFixed? (Variables|Default|GetBPC_Fix)))))