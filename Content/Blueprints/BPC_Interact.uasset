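; Interaction component for a Character owner that lets it use nearby actors implementing BPI_Interact.
; Capsule overlaps maintain an array of interactables and call begin/end interaction dispatchers, with begin gated by CanInteractMessage.
; A runtime screen-space WB_Interact prompt sits at the last entry, with text set for Note or Door tags on the first.
; IA_Interact messages the first entry, and DoneWithCurrent clears the array and prompt.
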(event Custom|HandleCapsuleOnBeginOverlap
  (params (OverlappedComponent :type Primitive%20Component%20Object%20Reference) (OtherActor :type Actor%20Object%20Reference) (OtherComp :type Primitive%20Component%20Object%20Reference) (OtherBodyIndex :type Integer) (bFromSweep :type Boolean) (SweepResult :type Hit%20Result%20Structure%20%28by%20ref%29))
  (if (Utilities|DoesObjectImplementInterface OtherActor "/Game/Blueprints/BPI_Interact.BPI_Interact_C")
    (Utilities|Array|AddUnique (Variables|Default|GetInteractableArray) OtherActor)
    (bind _boolparam (Class|BPIInteract|CanInteract?(Message) OtherActor))
    (if _boolparam
      (CallFunction|RenderInteractionWidget)
      (Default|CallOnInteractionBegin))))

(event Custom|HandleCapsuleOnEndOverlap
  (params (OverlappedComponent :type Primitive%20Component%20Object%20Reference) (OtherActor :type Actor%20Object%20Reference) (OtherComp :type Primitive%20Component%20Object%20Reference) (OtherBodyIndex :type Integer))
  (if (Utilities|DoesObjectImplementInterface OtherActor "/Game/Blueprints/BPI_Interact.BPI_Interact_C")
    (Utilities|Array|RemoveItem (Variables|Default|GetInteractableArray) OtherActor)
    (CallFunction|RenderInteractionWidget)
    (Default|CallOnInteractionEnd)))

(event Custom|DoneWithCurrent
  (Utilities|Array|Clear (Variables|Default|GetInteractableArray))
  (CallFunction|RenderInteractionWidget))

(event Input|EnhancedActionEvents|EnhancedInputActionIA_Interact
  (params (ActionValue :type Boolean) (ElapsedSeconds :type Float%20%28double-precision%29) (TriggeredSeconds :type Float%20%28double-precision%29) (InputAction :type Input%20Action%20Object%20Reference :default "/Game/FirstPerson/Input/Actions/IA_Interact.IA_Interact"))
  (:Started
    (Class|BPIInteract|Interact(Message) (Utilities|Array|Get(acopy) (Variables|Default|GetInteractableArray)) (Components|GetOwner))))

(event EventBeginPlay
  (bind _ascharacter (Utilities|Casting|CastToCharacter (Components|GetOwner)))
  (Collision|BindEventtoOnComponentBeginOverlap (Variables|/Script/Engine.Character|GetCapsuleComponent _ascharacter) (EventDispatchers|CreateEvent :!event Custom|HandleCapsuleOnBeginOverlap))
  (Collision|BindEventtoOnComponentEndOverlap (Variables|/Script/Engine.Character|GetCapsuleComponent _ascharacter) (EventDispatchers|CreateEvent :!event Custom|HandleCapsuleOnEndOverlap))
  (bind _returnvalue (Game|AddComponentbyClass (Components|GetOwner) "/Script/UMG.WidgetComponent" true))
  (Class|WidgetComponent|SetWidgetSpace _returnvalue "Screen")
  (Class|WidgetComponent|SetDrawSize _returnvalue "(X=250.000000,Y=60.000000)")
  (Variables|Default|SetInteractionWidget _returnvalue))

(fn RenderInteractionWidget
  (bind _interactionwidget (Variables|Default|GetInteractionWidget))
  (bind _interactablearray (Variables|Default|GetInteractableArray))
  (bind _output (Utilities|Array|Get(acopy) _interactablearray))
  (if (Utilities|Array|IsNotEmpty (Variables|Default|GetInteractableArray))
    (bind _returnvalue (UserInterface|CreateWidget "/Game/UI/WB_Interact.WB_Interact_C"))
    (UserInterface|SetWidget _interactionwidget _returnvalue)
    (Transformation|SetWorldLocation _interactionwidget (Transformation|GetActorLocation (CallFunction|GetActiveInteractable)) false false)
    (if (or (Actor|ActorHasTag _output "Note") (Actor|ActorHasTag _output "Door"))
      (Variables|/Script/UMG.TextBlock|SetText (Variables|/Game/UI/WB_Interact.WB_Interact_C|GetTextBlock_68 _returnvalue) "Press E to Use"))
    (else
      (UserInterface|SetWidget (Variables|Default|GetInteractionWidget) 0))))

(fn GetActiveInteractable
  (bind _interactablearray (Variables|Default|GetInteractableArray))
  (return (Utilities|Array|Get(acopy) _interactablearray (Utilities|Array|LastIndex _interactablearray))))