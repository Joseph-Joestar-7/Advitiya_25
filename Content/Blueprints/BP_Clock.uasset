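; BP_Clock is an interactable clock that the player can repair.
; Interacting calls Repair on its fix component, and CanInteract allows this only while that component is not yet fixed.
; When the component reports it has been fixed, the clock adds an audio component, triggers the player character's DoneMessage and clears the overlay material on its five meshes.
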(event HasBeenFixed(BPC_Fix)
  (AddComponent|AddAudioComponent false)
  (Class|BPIPlayer|Done(Message) (Game|GetPlayerCharacter 0))
  (Rendering|Material|SetOverlayMaterial (Variables|Default|GetdefaultMaterial) 0 :!class /Script/Engine.MeshComponent))

(event EventBeginPlay)

(event EventInteract
  (params (Interactor :type Actor%20Object%20Reference))
  (Default|Repair (Variables|Default|GetBPC_Fix)))

(fn ConstructionScript)

(fn CanInteract?
  (return (not (Variables|/Game/Blueprints/BPC_Fix.BPC_Fix_C|GetisFixed? (Variables|Default|GetBPC_Fix)))))