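; BP_Door is an interactable door that either swings open or, as the main door, shows the player an exit message.
; Interact works only while IsActivated is true, which CanInteract also reports, and branches on IsMainDoor to call the player character's ExitMessage or Open.
; Open runs once through a DoOnce, playing a Timeline that yaws the static mesh's relative rotation negatively from zero.
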(event Custom|Open
  (bind (_roll _pitch _yaw) (Math|Rotator|BreakRotator "0, 0, 0"))
  (Utilities|FlowControl|DoOnce false
    (:Completed
      (Variables|Default|SetNewVar (Transformation|GetActorRotation))
      (bind _newtrack_0 (Timeline|Timeline Play)
        (:Update
          (Transformation|SetRelativeRotation (Variables|Default|GetStaticMesh) (Math|Rotator|MakeRotator _roll _pitch (- _yaw _newtrack_0)) false false))))))

(event EventBeginPlay)

(event Collision|EventActorBeginOverlap
  (params (OtherActor :type Actor%20Object%20Reference)))

(event EventTick
  (params (DeltaSeconds :type Float%20%28single-precision%29)))

(event EventInteract
  (params (Interactor :type Actor%20Object%20Reference))
  (if (Variables|Default|GetisActivated?)
    (if (Variables|Default|GetisMainDoor?)
      (Class|BPIPlayer|Exit(Message) (Game|GetPlayerCharacter 0))
      (else
        (CallFunction|Open)))))

(fn ConstructionScript)

(fn CanInteract?
  (return (Variables|Default|GetisActivated?)))