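; BP_Monster is an AI monster that stalks the first-person player only while they are interacting and it is activated.
; It binds to the player's interaction-changed event to start AI MoveTo toward them or stop movement immediately.
; Tick uses a DoOnce with a delayed reset to add an audio component periodically while moving.
; Player overlap with its sphere while activated sends the player a jumpscare message.
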(event OnComponentBeginOverlap(Sphere)
  (params (OverlappedComponent :type Primitive%20Component%20Object%20Reference) (OtherActor :type Actor%20Object%20Reference) (OtherComp :type Primitive%20Component%20Object%20Reference) (OtherBodyIndex :type Integer) (bFromSweep :type Boolean) (SweepResult :type Hit%20Result%20Structure%20%28by%20ref%29))
  (bind _returnvalue (Game|GetPlayerCharacter 0))
  (if (and (== OtherActor _returnvalue) (Variables|Default|Getactivated?))
    (Class|BPIPlayer|Jumpscared(Message) _returnvalue)))

(event Custom|HandleInteractionChange
  (bind _output_get (Variables|Default|SetIs%20Interacting? (Variables|/Game/FirstPerson/Blueprints/BP_FirstPersonCharacter.BP_FirstPersonCharacter_C|GetbIsInteracting? (Variables|Default|GetAs%20BP%20First%20Person%20Character))))
  (if (and _output_get (Variables|Default|Getactivated?))
    (AI|AIMoveTo self "0, 0, 0" (Variables|Default|GetAs%20BP%20First%20Person%20Character) 1e+02 false)
    (else
      (Components|Movement|StopMovementImmediately (Variables|Character|GetCharacterMovement)))))

(event EventBeginPlay
  (bind _asbp_first_person_character (Utilities|Casting|CastToBP_FirstPersonCharacter (Game|GetPlayerCharacter 0)))
  (bind _output_get (Variables|Default|SetAs%20BP%20First%20Person%20Character _asbp_first_person_character))
  (EventDispatchers|BindEventtoOnInteractionChanged _output_get (delegate Custom|HandleInteractionChange)))

(event Collision|EventActorBeginOverlap
  (params (OtherActor :type Actor%20Object%20Reference)))

(event EventTick
  (params (DeltaSeconds :type Float%20%28single-precision%29))
  (if (> (Math|Vector|VectorLength (Transformation|GetVelocity)) 1e+01)
    (Utilities|FlowControl|DoOnce false :!label _label
      (:Completed
        (AddComponent|AddAudioComponent false)
        (Utilities|FlowControl|Delay 1.5)
        (goto _label Reset)))))

(fn ConstructionScript)