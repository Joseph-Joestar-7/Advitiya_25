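; BP_Fridge is an interactable fridge actor that the player can repair.
; Interacting calls Repair on its BPC_Fix component, and CanInteract allows interaction only while that component is not yet fixed.
; When the component fires HasBeenFixed, the fridge calls DoneMessage on the player character, adds an audio component and resets the mesh's overlay material.
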(event HasBeenFixed(BPC_Fix)
  (Class|BPIPlayer|Done(Message) (Game|GetPlayerCharacter 0))
  (AddComponent|AddAudioComponent false)
  (Rendering|Material|SetOverlayMaterial (Variables|Default|GetStaticMesh) 0 :!class /Script/Engine.MeshComponent))

(event EventBeginPlay)

(event Collision|EventActorBeginOverlap
  (params (OtherActor :type Actor%20Object%20Reference)))

(event EventTick
  (params (DeltaSeconds :type Float%20%28single-precision%29)))

(event EventInteract
  (params (Interactor :type Actor%20Object%20Reference))
  (Default|Repair (Variables|Default|GetBPC_Fix)))

(fn ConstructionScript)

(fn CanInteract?
  (return (not (Variables|/Game/Blueprints/BPC_Fix.BPC_Fix_C|GetisFixed? (Variables|Default|GetBPC_Fix)))))